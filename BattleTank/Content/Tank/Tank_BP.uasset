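; Player-controllable tank pawn Blueprint that wires its turret, barrel, tracks, aiming and movement components together.
; The construction script assigns meshes, track physical materials and the projectile class; BeginPlay initialises TankAiming and TankMovement and links the health bar widget to this tank.
; Input rotates the camera gimbal and spring arm, fires through TankAiming, and drives tracks either directly per side or through TankMovement's forward and turn intents.
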(event EventBeginPlay
  (Class|TankAimingComponent|Initialise (Variables|Default|GetTankAiming) (Variables|Default|GetBarrel) (Variables|Default|GetTurret))
  (Class|TankMovementComponent|Initialise (Variables|Default|GetTankMovement) (Variables|Default|GetLeft%20Track) (Variables|Default|GetRight%20Track))
  (CallFunction|IntialiseHealthBarWidget))

(event Input|ActionEvents|InputActionFire
  (params (Key :type Key%20Structure))
  ;[1 1 1] Aim and Fire Input Binding
  (:Pressed
    (Class|TankAimingComponent|Fire (Variables|Default|GetTankAiming))))

(event Input|AxisEvents|InputAxisAimAzimuth
  (params (AxisValue :type Float%20%28single-precision%29))
  ;[1 1 1] Aim and Fire Input Binding
  (Transformation|AddLocalRotation (Variables|Default|GetAzimuth%20Gimbal) (Math|Rotator|MakeRotator 0.0 0.0 AxisValue) false false))

(event Input|AxisEvents|InputAxisAimElevation
  (params (AxisValue :type Float%20%28single-precision%29))
  ;[1 1 1] Aim and Fire Input Binding
  (Transformation|AddLocalRotation (Variables|Default|GetSpringArm) (Math|Rotator|MakeRotator 0.0 AxisValue 0.0) false false))

(event Input|AxisEvents|InputAxisTurnRight
  (params (AxisValue :type Float%20%28single-precision%29))
  ;[1 1 1] Movement Input Binding
  (Class|TankMovementComponent|IntendTurnRight (Variables|Default|GetTankMovement) AxisValue))

(event Input|AxisEvents|InputAxisLeftTrackThrottle
  (params (AxisValue :type Float%20%28single-precision%29))
  ;[1 1 1] Movement Input Binding
  (Class|TankTrack|SetThrottle (Variables|Default|GetLeft%20Track) AxisValue))

(event Input|AxisEvents|InputAxisRightTrackThrottle
  (params (AxisValue :type Float%20%28single-precision%29))
  ;[1 1 1] Movement Input Binding
  (Class|TankTrack|SetThrottle (Variables|Default|GetRight%20Track) AxisValue))

(event Input|AxisEvents|InputAxisMoveForward
  (params (AxisValue :type Float%20%28single-precision%29))
  ;[1 1 1] Movement Input Binding
  (Class|TankMovementComponent|IntendMoveForward (Variables|Default|GetTankMovement) AxisValue))

(fn ConstructionScript
  (Components|StaticMesh|SetStaticMesh (Variables|Default|GetTurret) "/Game/Tank/tank_fbx_Turret.tank_fbx_Turret")
  (Components|StaticMesh|SetStaticMesh (Variables|Default|GetLeft%20Track) "/Game/Tank/tank_fbx_Track.tank_fbx_Track")
  (Components|StaticMesh|SetStaticMesh (Variables|Default|GetRight%20Track) "/Game/Tank/tank_fbx_Track.tank_fbx_Track")
  (Class|PrimitiveComponent|SetPhysMaterialOverride (Variables|Default|GetLeft%20Track) "/Game/Tank/track.Track")
  (Class|PrimitiveComponent|SetPhysMaterialOverride (Variables|Default|GetRight%20Track) "/Game/Tank/track.Track")
  (Variables|/Script/BattleTank.TankAimingComponent|SetprojectileBlueprint (Variables|Default|GetTankAiming) "/Game/Projectile/Projectile_BP.Projectile_BP_C"))

(fn IntialiseHealthBarWidget
  (bind _ashealth_bar_bp (Utilities|Casting|CastToHealthBar_BP (UserInterface|GetUserWidgetObject (Variables|Default|GetHealth%20Bar))))
  (Variables|/Game/UI/HealthBar_BP.HealthBar_BP_C|SetOwningTank _ashealth_bar_bp self))